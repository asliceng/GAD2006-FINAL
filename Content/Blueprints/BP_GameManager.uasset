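; BP_GameManager is the game manager Blueprint that drives the UI for a turn-based game.
; On BeginPlay it creates and stores the game-state widget, whose active player label updates on PlayerChanged from the current player's display name.
; WarningPopUp briefly shows that widget's warning using a delay, and OnGameOverScreen creates a separate game-over widget announcing the winner.
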(event EventBeginPlay
  (bind _returnvalue (UserInterface|CreateWidget "/Game/Blueprints/UMG/WBP_GameStates.WBP_GameStates_C"))
  (bind _output_get (Variables|Default|SetWBP_GameStates _returnvalue))
  (UserInterface|Viewport|AddtoViewport _output_get 0))

(event EventPlayerChanged
  (Variables|/Script/UMG.TextBlock|SetText (Variables|/Game/Blueprints/UMG/WBP_GameStates.WBP_GameStates_C|GetActivePlayer (Variables|Default|GetWBP_GameStates)) (Utilities|Text|ToText(String) (Utilities|String|Append (Utilities|GetDisplayName (Class|GameManager|GetCurrentPlayer)) " Turn"))))

(event EventWarningPopUp
  (bind _wbp_gamestates (Variables|Default|GetWBP_GameStates))
  (bind _warning (Variables|/Game/Blueprints/UMG/WBP_GameStates.WBP_GameStates_C|GetWarning _wbp_gamestates))
  (Variables|/Script/UMG.Widget|SetVisibility _warning "Visible")
  (Utilities|FlowControl|Delay 2.0)
  (Variables|/Script/UMG.Widget|SetVisibility _warning "Collapsed"))

(event EventOnGameOverScreen
  (bind _returnvalue (UserInterface|CreateWidget "/Game/Blueprints/UMG/WBP_GameOver.WBP_GameOver_C"))
  (Rendering|Components|TextRender|SetText (Variables|/Game/Blueprints/UMG/WBP_GameOver.WBP_GameOver_C|GetWinner _returnvalue) (Utilities|Text|ToText(String) (Utilities|String|Append (Utilities|GetDisplayName (Variables|Default|GetWinnerPlayer)) " Won!")))
  (UserInterface|Viewport|AddtoViewport _returnvalue 0))

(fn ConstructionScript)